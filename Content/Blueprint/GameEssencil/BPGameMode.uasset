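; Multiplayer game mode that tracks joining and leaving player controllers, spawns their characters and handles level changes.
; Each new player gets a ThirdPersonCharacter at a random SpawnPosition actor and possesses it, except in MainMenu.
; ChangeLevel shows the game instance's loading screen, then runs servertravel through a console command.
; The loop meant to show every player's loading screen is empty, its call left unconnected.
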(event Custom|ChangeLevel
  (params (Level%20Name :type Name))
  ;[1 1 1] ChangeLevel
  (bind _asbpgame_instance (Utilities|Casting|CastToBPGameInstance (Game|GetGameInstance)))
  (Default|ShowLoadingScreen _asbpgame_instance)
  (CallFunction|ShowAllPlayerLodingScreen)
  (Development|ExecuteConsoleCommand (Utilities|String|Append "servertravel " (Utilities|String|ToString(Name) Level%20Name)) (Game|GetPlayerController 0)))

(event Custom|SpawnPawn
  (params (PlayerController :type BP%20Player%20Controller%20Object%20Reference) (Number :type Integer))
  (bind _returnvalue (Game|GetCurrentLevelName true))
  (if (not (Utilities|Enum|Equal(Enum) _returnvalue "MainMenu"))
    (bind _outactors (Actor|GetAllActorsOfClass "/Game/Blueprint/SpawnPosition.SpawnPosition_C"))
    (bind _returnvalue_2 (Game|SpawnActorfromClass "/Game/ThirdPersonBP/Blueprints/ThirdPersonCharacter.ThirdPersonCharacter_C" (Transformation|GetActorTransform (Utilities|Array|Get(acopy) _outactors (Math|Random|RandomIntegerinRange 0 (- (Utilities|Array|Length _outactors) 1)))) "Undefined" 0 0))
    (Pawn|Possess PlayerController _returnvalue_2)))

(event Custom|ShowAllPlayerLodingScreen
  ;[1 1 1] ShowAllPlayerLodingScreen
  (for _array_element (Variables|Default|Getplayers)
    _))

(event EventOnLogout
  (params (ExitingController :type Controller%20Object%20Reference))
  (bind _asbpplayer_controller (Utilities|Casting|CastToBPPlayerController ExitingController))
  (Utilities|Array|RemoveItem (Variables|Default|Getplayers) _asbpplayer_controller)
  (Math|Integer|DecrementInt (Variables|Default|GetplayerCount)))

(event EventHandleStartingNewPlayer
  (params (NewPlayer :type Player%20Controller%20Object%20Reference))
  (bind _asbpplayer_controller (Utilities|Casting|CastToBPPlayerController NewPlayer))
  (Utilities|Array|Add (Variables|Default|Getplayers) _asbpplayer_controller)
  (bind _result (Math|Integer|IncrementInt (Variables|Default|GetplayerCount))
    (:%20%20
      (CallFunction|SpawnPawn _asbpplayer_controller _result))))

(fn ConstructionScript)